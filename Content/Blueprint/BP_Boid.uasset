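; BP_Boid is a boid actor with a cube that visually reflects the player assigned as its Leader.
; On a leader change, it casts the Leader to BP_Player and copies the first material of that player's cube onto its own.
; It picks a random rotation rate at BeginPlay and spins the cube each Tick while the Leader is valid.
; This Blueprint's graphs contain no flocking or movement logic.
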(event `self.OnLeaderChange`
  (bind _asbp_player (cast `/Game/Blueprint/BP_Player` (`self.leader`)))
  (`PrimitiveComponent.SetMaterial` (`self.Cube`) 0 (`|GetArrayItem` (`MeshComponent.GetMaterials` (`/Game/Blueprint/BP_Player.Cube` _asbp_player)))))

(event `self.ReceiveTick`
  (params (DeltaSeconds :type "Float (single-precision)"))
  (`/Engine/EditorBlueprintResources/StandardMacros.IsValid` (`self.leader`)
    (:`Is Valid`
      (`SceneComponent.K2_AddLocalRotation` (`self.Cube`) (* (`self.RandomRoate`) DeltaSeconds) false false))))

(event `self.ReceiveBeginPlay`
  (set `self.RandomRoate` (`KismetMathLibrary.MakeRotator` (`KismetMathLibrary.RandomFloatInRange` 0.0 360.0) (`KismetMathLibrary.RandomFloatInRange` 0.0 360.0) (`KismetMathLibrary.RandomFloatInRange` 0.0 360.0))))

(fn `UserConstructionScript`)