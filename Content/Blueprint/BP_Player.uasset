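; BP_Player is the player Blueprint, handling laser-shot feedback and per-player UI.
; Shoot events stretch a beam emitter from ShootPoint to a position or actor and play a sound.
; Actor hits add an explosion effect and sound and flash the aim widget's hit marker.
; On possession it sets the name widget from the network slot name and creates the aim widget only for player controller 0.
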(event `PlayExplosionSound`
  (params (Location :type "Vector Structure"))
  (`GameplayStatics.PlaySoundAtLocation` "/Game/Sound/Black_Cow_Game_Sound_Pack_Ver0_2/Creature_Ai_Soldier/Ai_Soldier_Die/Ai_Soldier_Sword_Die_01.Ai_Soldier_Sword_Die_01" Location (struct) 1.0 1.0 0.3 null null null))

(event `PlayShootSound`
  (`GameplayStatics.PlaySoundAtLocation` "/Game/Sound/Black_Cow_Game_Sound_Pack_Ver0_2/Creature_Ai_Soldier/Ai_Soldier_Laser_Attack/Ai_Soldier_Laser_Attack_01.Ai_Soldier_Laser_Attack_01" (`self.K2_GetActorLocation`) (struct) 1.0 1.0 0.3 null null null))

(event `SpawnLaser`
  (params (Point :type "Vector Structure"))
  (bind _returnvalue (`GameplayStatics.SpawnEmitterAtLocation` "/Game/Resources/Enemy/AI/P_Laser2.P_Laser2" (`SceneComponent.K2_GetComponentLocation` (`self.ShootPoint`)) (`self.GetControlRotation`)))
  (for _index (range 11)
    (`ParticleSystemComponent.SetBeamTargetPoint` _returnvalue _index Point _index)))

(event `self.ShootParticleToVector`
  (params (pos :type "Vector Structure"))
  (`self.SpawnLaser` pos)
  (`self.PlayShootSound`))

(event `self.ShootParticleToActor`
  (params (actor :type "Actor Object Reference"))
  (bind _returnvalue (`self.K2_GetActorLocation` actor))
  (bind _aimwidget (`self.AimWidget`))
  (`self.SpawnLaser` _returnvalue)
  (`GameplayStatics.SpawnEmitterAtLocation` "/Game/Resources/Enemy/AI/P_AI_Explod.P_AI_Explod" _returnvalue (`KismetMathLibrary.RandomRotator` true) (3.0 3.0 3.0))
  (`self.PlayShootSound`)
  (`self.PlayExplosionSound` _returnvalue)
  (`/Engine/EditorBlueprintResources/StandardMacros.IsValid` _aimwidget
    (:`Is Valid`
      (`/Game/Blueprint/UI/PlayerAim.ShowHitAim` _aimwidget))))

(event `self.ReceivePossessed`
  (params (NewController :type "Controller Object Reference"))
  (bind _returnvalue (`GameplayStatics.GetPlayerController` 0))
  (bind _netbasecp (`self.NetBaseCP`))
  (`|ExecutionSequence`
    (:`then_0`
      (bind _asplayer_widget (cast `/Game/Blueprint/UI/PlayerWidget` (`WidgetComponent.GetUserWidgetObject` (`self.Widget`))))
      (`/Game/Blueprint/UI/PlayerWidget.SetID` _asplayer_widget (`InGameNetworkProcessor.GetSlotName` (`NetworkBaseCP.GetInGameNetworkProcessor` _netbasecp) (`NetworkBaseCP.GetCurrentAuthority` _netbasecp))))
    (:`then_1`
      (if (== NewController _returnvalue)
        (bind _returnvalue_2 (`|CreateWidget` "/Game/Blueprint/UI/PlayerAim.PlayerAim_C" _returnvalue))
        (`UserWidget.AddToViewport` _returnvalue_2 0)
        (set `self.AimWidget` _returnvalue_2)))))

(fn `UserConstructionScript`)